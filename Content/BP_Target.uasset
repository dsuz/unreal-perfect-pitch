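; BP_Target manages nine physics targets for a ball-throwing game, handling hit sounds, reset, knock-down detection and scoring.
; An overlap with its box blends the player camera to this actor.
; A looping timer polls until bodies sleep, forcing sleep after repeated checks, then hides targets below the drop height.
; Score grows with the square of the dropped count, shows in a score widget and animates on the main UI via timeline.
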(event OnComponentBeginOverlap(BoxCollision)
  (params (OverlappedComponent :type Primitive%20Component%20Object%20Reference) (OtherActor :type Actor%20Object%20Reference) (OtherComp :type Primitive%20Component%20Object%20Reference) (OtherBodyIndex :type Integer) (bFromSweep :type Boolean) (SweepResult :type Hit%20Result%20Structure%20%28by%20ref%29))
  (Development|PrintString "A ball overlapped target.")
  (CallFunction|SwitchtoTargetCamera))

(event Custom|UpdateScore
  (params (NewScore :type Integer) (NewBallCount :type Integer) (LastScore :type Integer))
  (bind _alpha (Timeline|Timeline PlayFromStart)
    (:Update
      (Default|UpdateScoreandBallCount (Variables|/Game/BP_GameInstance.BP_GameInstance_C|GetMainUI (Variables|Default|GetGameInstance)) (Math|Float|Truncate (Math|Float|Lerp (Math|Conversions|ToFloat(Integer) LastScore) (Math|Conversions|ToFloat(Integer) NewScore) _alpha)) NewBallCount))))

(event EventBeginPlay
  (bind _asbp_game_instance (Utilities|Casting|CastToBP_GameInstance (Game|GetGameInstance)))
  (Variables|Default|SetGameInstance _asbp_game_instance))

(event Collision|EventHit
  (params (MyComp :type Primitive%20Component%20Object%20Reference) (Other :type Actor%20Object%20Reference) (OtherComp :type Primitive%20Component%20Object%20Reference) (bSelfMoved :type Boolean) (HitLocation :type Vector :default "0, 0, 0") (HitNormal :type Vector :default "0, 0, 0") (NormalImpulse :type Vector :default "0, 0, 0") (Hit :type Hit%20Result%20Structure%20%28by%20ref%29))
  (Utilities|Casting|CastToBP_Ball Other)
  (if (Physics|IsSimulatingPhysics MyComp "None")
    (Audio|PlaySoundatLocation (Variables|Default|GetTargetHit) HitLocation "0, 0, 0" 1.0 1.0 0.0 0 0 0 0)
    (else
      (Audio|PlaySoundatLocation (Variables|Default|GetHeavyHit) HitLocation "0, 0, 0" 1.0 1.0 0.0 0 0 0 0))))

(fn ConstructionScript
  (CallFunction|Initialize))

(fn Initialize
  (bind _output_get (Variables|Default|SetTargetReferences (Utilities|Array|MakeArray (Variables|Default|GetTarget1) (Variables|Default|GetTarget2) (Variables|Default|GetTarget3) (Variables|Default|GetTarget4) (Variables|Default|GetTarget5) (Variables|Default|GetTarget6) (Variables|Default|GetTarget7) (Variables|Default|GetTarget8) (Variables|Default|GetTarget9))))
  (for _index (range 0 (Utilities|Array|LastIndex _output_get))
    (Utilities|Array|SetArrayElem (Variables|Default|GetTargetInitialPositions) _index (Transformation|GetWorldLocation (Utilities|Array|Get(acopy) (Variables|Default|GetTargetReferences) _index)))))

(fn ResetTarget
  (for _index (range 0 (Utilities|Array|LastIndex (Variables|Default|GetTargetReferences)))
    (Rendering|SetVisibility (Utilities|Array|Get(acopy) (Variables|Default|GetTargetReferences) _index) true false)
    (Physics|SetSimulatePhysics (Utilities|Array|Get(acopy) (Variables|Default|GetTargetReferences) _index) true)
    (Collision|SetCollisionEnabled (Utilities|Array|Get(acopy) (Variables|Default|GetTargetReferences) _index) "QueryAndPhysics")
    (Class|PrimitiveComponent|PutRigidBodytoSleep (Utilities|Array|Get(acopy) (Variables|Default|GetTargetReferences) _index) "None")
    (Transformation|SetWorldRotation (Utilities|Array|Get(acopy) (Variables|Default|GetTargetReferences) _index) "0, 0, 0" false false)
    (Transformation|SetWorldLocation (Utilities|Array|Get(acopy) (Variables|Default|GetTargetReferences) _index) (Utilities|Array|Get(acopy) (Variables|Default|GetTargetInitialPositions) _index) false false)))

(fn WaitUntilTargetPhysics
  (bind _checktargetinterval (Variables|Default|GetCheckTargetInterval))
  (bind _returnvalue (Utilities|Time|SetTimerbyFunctionName 0 "IsTargetPhysicsAwake" _checktargetinterval true _checktargetinterval))
  (Variables|Default|SetTimer _returnvalue))

(fn IsTargetPhysicsAwake
  (for _array_element (Variables|Default|GetTargetReferences)
    (bind _output_get (LocalVariables|SetCurrentCheckingTarget _array_element))
    (if (and (Class|PrimitiveComponent|IsAnyRigidBodyAwake _output_get) (Class|SceneComponent|IsAnySimulatingPhysics _output_get))
      (bind _returnvalue (Physics|GetPhysicsLinearVelocity _array_element "None"))
      (Development|PrintString (Utilities|String|BuildString(Vector) (Utilities|String|BuildString(Object) "" "" _array_element " is awake. ") "Linear Velocity: " _returnvalue))
      (bind _result (Math|Integer|IncrementInt (Variables|Default|GetCheckTargetPhysicsRetryCounter))
        (:%20%20
          (Development|PrintString (Utilities|String|BuildString(Integer) "" "Physics Check Count: " _result))
          (if (>= (Variables|Default|GetCheckTargetPhysicsRetryCounter) (Variables|Default|GetMaxCheckTargetPhysicsCount))
            (Class|PrimitiveComponent|PutRigidBodytoSleep (LocalVariables|GetCurrentCheckingTarget) "None")
            (Development|PrintString (Utilities|String|BuildString(Object) "" "Forced " (LocalVariables|GetCurrentCheckingTarget) " to sleep")))
          (return)))))
  (Development|PrintString "All targets are sleeping")
  (Utilities|Time|ClearandInvalidateTimerbyHandle (Variables|Default|GetTimer))
  (CallFunction|PickupHitTargets)
  (Variables|Default|SetCheckTargetPhysicsRetryCounter 0)
  (return))

(fn PickupHitTargets
  (LocalVariables|SetCounter 0)
  (for _array_element (Variables|Default|GetTargetReferences)
    (LocalVariables|SetElement _array_element)
    (if (and (Rendering|IsVisible _array_element) (< (.Z (Math|Vector|BreakVector (Transformation|GetWorldLocation _array_element))) (Variables|Default|GetDroppedHeight)))
      (Development|PrintString (Utilities|String|BuildString(Object) "" "" _array_element " is dropped"))
      (LocalVariables|SetCounter (+ (LocalVariables|GetCounter) 1))
      (Rendering|SetVisibility (LocalVariables|GetElement) false false)
      (Physics|SetSimulatePhysics (LocalVariables|GetElement) false)
      (Collision|SetCollisionEnabled (LocalVariables|GetElement) "NoCollision")))
  (Development|PrintString (Utilities|String|BuildString(Integer) "" "" (LocalVariables|GetCounter) " tagets dropped"))
  (CallFunction|CalculateScore (LocalVariables|GetCounter))
  (return (LocalVariables|GetCounter)))

(fn CalculateScore
  (params (DroppedTargetCount :type Integer))
  (bind _gameinstance (Variables|Default|GetGameInstance))
  (bind _gameinstance_2 (Variables|Default|GetGameInstance))
  (LocalVariables|SetLastScore (Variables|/Game/BP_GameInstance.BP_GameInstance_C|GetScore (Variables|Default|GetGameInstance)))
  (LocalVariables|SetHitTargetCount DroppedTargetCount)
  (LocalVariables|SetNewScore (|((count*count)*baseScore) (LocalVariables|GetHitTargetCount) (Variables|/Game/BP_GameInstance.BP_GameInstance_C|GetBaseScore (Variables|Default|GetGameInstance))))
  (bind _returnvalue (UserInterface|CreateWidget "/Game/WBP_Score.WBP_Score_C"))
  (bind _output_get (Variables|/Game/BP_GameInstance.BP_GameInstance_C|SetScoreUI _gameinstance_2 _returnvalue))
  (Default|SetValues _output_get (LocalVariables|GetHitTargetCount) (Variables|/Game/BP_GameInstance.BP_GameInstance_C|GetBaseScore _gameinstance_2) (LocalVariables|GetNewScore) (LocalVariables|GetHitTargetCount))
  (UserInterface|Viewport|AddtoViewport (Variables|/Game/BP_GameInstance.BP_GameInstance_C|GetScoreUI (Variables|Default|GetGameInstance)) 0)
  (Default|AddScore (Variables|Default|GetGameInstance) (LocalVariables|GetNewScore))
  (CallFunction|UpdateScore (Variables|/Game/BP_GameInstance.BP_GameInstance_C|GetScore _gameinstance) (Variables|/Game/BP_GameInstance.BP_GameInstance_C|GetBallCount _gameinstance) (LocalVariables|GetLastScore)))

(fn GetUndroppedTargets
  (LocalVariables|SetCounter 0)
  (for _array_element (Variables|Default|GetTargetReferences)
    (if (Rendering|IsVisible _array_element)
      (Math|Integer|IncrementInt (LocalVariables|GetCounter))))
  (Development|PrintString (Utilities|String|BuildString(Integer) "" "Targets Count: " (LocalVariables|GetCounter)))
  (return (LocalVariables|GetCounter)))

(fn SwitchtoTargetCamera
  (Game|Player|SetViewTargetwithBlend (Game|GetPlayerController 0) self 0.5 "VTBlend_EaseOut" 1.5 false))