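; Player pawn for a ball-pitching game, where the player aims and throws a ball from the character's hand.
; Mouse input applies force to an Aim component, and the camera rotates to look at it.
; Pitch hides the held ball and launches a spawned BP_Ball from a hand socket toward Aim, scaling speed by power.
; Other functions toggle control flags, destroy the thrown ball, and ready a new one while updating game-instance status.
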(event EventBeginPlay
  (Variables|Default|SetDefaultAimLocation (Transformation|GetWorldLocation (Variables|Default|GetAim))))

(event Input|AxisEvents|InputAxisMouseHorizontal
  (params (AxisValue :type Float%20%28single-precision%29))
  (Physics|AddForce (Variables|Default|GetAim) (* (Variables|Default|GetCameraMoveSpeed) (Math|Vector|MakeVector 0.0 AxisValue (stale Input|AxisEvents|InputAxisMouseVertical AxisValue))) "None" false)
  (Transformation|SetWorldRotation (Variables|Default|GetCamera) (Math|Rotator|FindLookatRotation (Transformation|GetWorldLocation (Variables|Default|GetCamera)) (Transformation|GetWorldLocation (Variables|Default|GetAim))) false false))

(event Input|AxisEvents|InputAxisMouseVertical
  (params (AxisValue :type Float%20%28single-precision%29))
  (Physics|AddForce (Variables|Default|GetAim) (* (Variables|Default|GetCameraMoveSpeed) (Math|Vector|MakeVector 0.0 (stale Input|AxisEvents|InputAxisMouseHorizontal AxisValue) AxisValue)) "None" false)
  (Transformation|SetWorldRotation (Variables|Default|GetCamera) (Math|Rotator|FindLookatRotation (Transformation|GetWorldLocation (Variables|Default|GetCamera)) (Transformation|GetWorldLocation (Variables|Default|GetAim))) false false))

(fn ConstructionScript)

(fn TestFunction
  (Development|PrintString (Utilities|GetDisplayName self)))

(fn Pitch
  (params (Power :type Float%20%28double-precision%29))
  (Rendering|SetVisibility (Variables|Default|GetBall) false false)
  (bind _returnvalue (Game|SpawnActorfromClass "/Game/BP_Ball.BP_Ball_C" (Math|Conversions|ToTransform(Vector) (Transformation|GetSocketLocation (Actor|GetComponentbyClass "/Script/Engine.SkeletalMeshComponent") "middle_03_r")) "Undefined" "MultiplyWithRoot" 0 0))
  (Variables|Default|SetThrownBall _returnvalue)
  (Physics|SetPhysicsLinearVelocity (Variables|/Game/BP_Ball.BP_Ball_C|GetStaticMesh _returnvalue) (* (|(((max-min)*ratio)+min) (Variables|Default|GetMaxPower) (Variables|Default|GetMinPower) Power) (Math|Vector|GetUnitDirection(Vector) (Transformation|GetWorldLocation (Variables|/Script/Engine.Actor|GetRootComponent _returnvalue)) (Transformation|GetWorldLocation (Variables|Default|GetAim)))) false "None"))

(fn GetNewBall
  (Development|SetHiddeninGame (Variables|Default|GetBall) false false)
  (Class|SubmixEffectDelayStatics|SetDelayLength (Variables|Default|GetDelay%20Settings) (Variables|Default|GetWaitSecondsWhenGetNewBall))
  (Development|PrintString "Play!")
  (bind _asbp_game_instance (Utilities|Casting|CastToBP_GameInstance (Game|GetGameInstance)))
  (Default|ChangeStatus _asbp_game_instance "NewEnumerator4"))

(fn BeginActionControl
  (Variables|Default|SetActionControllable true))

(fn EndControls
  (Variables|Default|SetActionControllable false)
  (Variables|Default|SetAxisControllable false))

(fn BeginAxisControl
  (Variables|Default|SetAxisControllable true))

(fn PickupThrownBall
  (Actor|DestroyActor (Variables|Default|GetThrownBall)))