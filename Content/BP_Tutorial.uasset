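; BP_Tutorial plays queued tutorial voice lines when tutorials are enabled in BP_GameInstance.
; PlayTutorial adds a voice key to a queue capped at MaxQueueSize.
; Each tick, if the audio component is idle, it looks up the first queued key in TutorialVoiceMap, plays that sound and removes it, so lines play in order without overlapping.
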(event EventTick
  (params (DeltaSeconds :type Float%20%28single-precision%29))
  (if (Variables|/Game/BP_GameInstance.BP_GameInstance_C|GetPlayTutorial (Variables|Default|GetGameInstance))
    (if (not (Audio|Components|Audio|IsPlaying (Variables|Default|GetAudio)))
      (if (> (Utilities|Array|Length (Variables|Default|GetQueue)) 0)
        (Audio|Components|Audio|SetSound (Variables|Default|GetAudio) (.Value (Utilities|Map|Find (Variables|Default|GetTutorialVoiceMap) (Utilities|Array|Get(acopy) (Variables|Default|GetQueue)))))
        (Audio|Components|Audio|Play (Variables|Default|GetAudio) 0.0)
        (Utilities|Array|RemoveIndex (Variables|Default|GetQueue))))))

(event EventBeginPlay
  (bind _asbp_game_instance (Utilities|Casting|CastToBP_GameInstance (Game|GetGameInstance)))
  (Variables|Default|SetGameInstance _asbp_game_instance))

(fn ConstructionScript)

(fn PlayTutorial
  (params (Voice :type E_TutorialVoice%20Enum :default "NewEnumerator0"))
  (if (Variables|/Game/BP_GameInstance.BP_GameInstance_C|GetPlayTutorial (Variables|Default|GetGameInstance))
    (if (not (>= (Utilities|Array|Length (Variables|Default|GetQueue)) (Variables|Default|GetMaxQueueSize)))
      (Utilities|Array|Add (Variables|Default|GetQueue) Voice))))